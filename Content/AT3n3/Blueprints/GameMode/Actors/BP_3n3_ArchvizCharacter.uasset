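; First-person player character for architectural visualization walkthroughs, driven by Enhanced Input through the IMC_ArchViz mapping context.
; It handles movement and sensitivity-scaled look, with run and crouch as toggles that change walk speed and animate camera height.
; The zoom toggle runs timelines that animate the camera's focal length and update post-process settings.
; Zooming also animates manual focus scaled by HittingDistance, then restores a fixed focus distance on exit.
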(event Custom|AutoFocus
  ;[1 1 1] Camera AutoFocus
  (bind _distance (Timeline|FocusDistance Play)
    (:Update
      (Variables|/Script/CinematicCamera.CineCameraComponent|SetFocusSettings (Variables|Default|GetFirstPersonCamera) (Utilities|Struct|MakeCameraFocusSettings "Manual" (* _distance (Variables|Default|GetHittingDistance)))))))

(event Custom|EndFocus
  ;[1 1 1] Camera AutoFocus
  (Variables|/Script/CinematicCamera.CineCameraComponent|SetFocusSettings (Variables|Default|GetFirstPersonCamera) (Utilities|Struct|MakeCameraFocusSettings "Manual" 1e+02)))

(event Input|EnhancedActionEvents|EnhancedInputActionIA_Move
  (params (ActionValue :type Vector%202D%20Structure) (ElapsedSeconds :type Float%20%28double-precision%29) (TriggeredSeconds :type Float%20%28double-precision%29) (InputAction :type Input%20Action%20Object%20Reference :default "/Game/AT3n3/Blueprints/GameMode/Inputs/IA_Move.IA_Move"))
  ;[1 1 1] Movement
  (Pawn|Input|AddMovementInput (Transformation|GetActorRightVector) (.x ActionValue) false)
  (Pawn|Input|AddMovementInput (Transformation|GetActorForwardVector) (.y ActionValue) false))

(event Input|EnhancedActionEvents|EnhancedInputActionIA_Crouch
  (params (ActionValue :type Boolean) (ElapsedSeconds :type Float%20%28double-precision%29) (TriggeredSeconds :type Float%20%28double-precision%29) (InputAction :type Input%20Action%20Object%20Reference :default "/Game/AT3n3/Blueprints/GameMode/Inputs/IA_Crouch.IA_Crouch"))
  ;[1 1 1] Crouch
  (:Started
    (Utilities|FlowControl|FlipFlop
      (:A
        (bind _speed (Timeline|CrouchMovement PlayFromStart)
          (:Update
            (Transformation|SetRelativeLocation (Variables|Default|GetFirstPersonCamera) (Math|Vector|MakeVector 0.0 0.0 _speed) false false))))
      (:B
        (Timeline|CrouchMovement ReverseFromEnd)))))

(event Input|EnhancedActionEvents|EnhancedInputActionIA_Run
  (params (ActionValue :type Boolean) (ElapsedSeconds :type Float%20%28double-precision%29) (TriggeredSeconds :type Float%20%28double-precision%29) (InputAction :type Input%20Action%20Object%20Reference :default "/Game/AT3n3/Blueprints/GameMode/Inputs/IA_Run.IA_Run"))
  (bind _charactermovement (Variables|Character|GetCharacterMovement))
  ;[1 1 1] Run
  (:Started
    (Utilities|FlowControl|FlipFlop
      (:A
        (Variables|/Script/Engine.CharacterMovementComponent|SetMaxWalkSpeed _charactermovement 2.5e+02))
      (:B
        (Variables|/Script/Engine.CharacterMovementComponent|SetMaxWalkSpeed _charactermovement 7e+01)))))

(event Input|EnhancedActionEvents|EnhancedInputActionIA_Look
  (params (ActionValue :type Vector%202D%20Structure) (ElapsedSeconds :type Float%20%28double-precision%29) (TriggeredSeconds :type Float%20%28double-precision%29) (InputAction :type Input%20Action%20Object%20Reference :default "/Game/AT3n3/Blueprints/GameMode/Inputs/IA_Look.IA_Look"))
  (bind _mousesensitivity (Variables|Default|GetMouseSensitivity))
  ;[1 1 1] Mouse
  (Pawn|Input|AddControllerYawInput (* (.x ActionValue) _mousesensitivity))
  (Pawn|Input|AddControllerPitchInput (* (.y ActionValue) _mousesensitivity)))

(event Input|EnhancedActionEvents|EnhancedInputActionIA_Zoom
  (params (ActionValue :type Boolean) (ElapsedSeconds :type Float%20%28double-precision%29) (TriggeredSeconds :type Float%20%28double-precision%29) (InputAction :type Input%20Action%20Object%20Reference :default "/Game/AT3n3/Blueprints/GameMode/Inputs/IA_Zoom.IA_Zoom"))
  (bind _firstpersoncamera (Variables|Default|GetFirstPersonCamera))
  ;[1 1 1] Camera Zoom
  (:Started
    (Utilities|FlowControl|FlipFlop
      (:A
        (Utilities|FlowControl|Sequence
          (:then_0
            (bind _focallenght (Timeline|Zoom Play)
              (:Update
                (Variables|/Script/CinematicCamera.CineCameraComponent|SetCurrentFocalLength _firstpersoncamera _focallenght))))
          (:then_1
            (Timeline|Timeline Play
              (:Update
                (Variables|/Script/Engine.CameraComponent|SetPostProcessSettings _firstpersoncamera ""))))
          (:then_2
            (CallFunction|AutoFocus))))
      (:B
        (Utilities|FlowControl|Sequence
          (:then_0
            (Timeline|Zoom Reverse))
          (:then_1
            (Timeline|Timeline Reverse))
          (:then_2
            (CallFunction|EndFocus)))))))

(event EventBeginPlay
  ;[1 1 1] Enhanced Input
  (bind _asplayer_controller (Utilities|Casting|CastToPlayerController (Pawn|GetController)))
  (Utilities|IsValid (PlayerController|LocalPlayerSubsystems|GetEnhancedInputLocalPlayerSubsystem _asplayer_controller)
    (:Is%20Valid
      (Input|AddMappingContext (PlayerController|LocalPlayerSubsystems|GetEnhancedInputLocalPlayerSubsystem _asplayer_controller) "/Game/AT3n3/Blueprints/GameMode/Inputs/IMC_ArchViz.IMC_ArchViz" 0 "(bIgnoreAllPressedKeysUntilRelease=True,bForceImmediately=False,bNotifyUserSettings=False)"))))

(fn ConstructionScript)